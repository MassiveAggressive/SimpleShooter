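; GeneralFunctions is a set of shared helper functions for reaching common player and game objects.
; GetHitResult runs a complex trace under the first player's cursor against one object type and returns the hit location and actor.
; GetPlayerControllerBase casts the indexed controller to BP_PlayerControllerBase.
; GetWidget and GetStatsComponent avoid casts by sending getter messages to the game mode and indexed player controller, respectively.
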(fn `GetHitResult`
  (returns (Location :type "Vector Structure") (HitActor :type "Actor Object Reference"))
  (bind (_bblockinghit _binitialoverlap _time _distance _location _impactpoint _normal _impactnormal _physmat _hitactor) (`GameplayStatics.BreakHitResult` (`PlayerController.GetHitResultUnderCursorForObjects` (`GameplayStatics.GetPlayerController` null) (`|MakeArray` "ObjectTypeQuery12" :!type "EObjectTypeQuery Enum") true)))
  (return _location _hitactor))

(fn `GetPlayerControllerBase`
  (params (PlayerIndex :type Integer))
  (returns (PlayerController :type "/Game/Blueprint/Player/BP_PlayerControllerBase Object Reference"))
  (bind _asbp_player_controller_base (cast `/Game/Blueprint/Player/BP_PlayerControllerBase` (`GameplayStatics.GetPlayerController` null PlayerIndex)))
  (return _asbp_player_controller_base))

(fn `GetStatsComponent`
  (params (PlayerIndex :type Integer))
  (returns (StatsComponent :type "/Game/Blueprint/Stat/AC_Stats Object Reference"))
  (bind _statscomponent (message `/Game/Blueprint/Player/Interface/BPI_PlayerController.GetStatsComponent` (`GameplayStatics.GetPlayerController` null PlayerIndex)))
  (return _statscomponent))

(fn `GetWidget`
  (returns (Widget :type "UserWidget Object Reference"))
  (bind _widget (message `/Game/Blueprint/GameMode/Interface/BPI_GameMode.GetWidget` (`GameplayStatics.GetGameMode` null)))
  (return _widget))