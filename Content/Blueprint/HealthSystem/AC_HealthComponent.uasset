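; An actor component that tracks health and shield for its owner in the health system.
; On BeginPlay it fills current values to their maximums and, only for the player pawn, binds to the stats component's update event.
; StatsUpdated reads new maximum health and shield from the stats map.
; AddHealth applies damage or regeneration with clamping and calls the owner's destroy at zero health, leaving shield untouched.
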(event `self.ReceiveBeginPlay`
  (if (== (`self.GetOwner`) (`GameplayStatics.GetPlayerPawn` 0))
    (add `/Game/Blueprint/StatSystem/AC_Stats.StatsUpdated` (`/Game/Blueprint/GeneralFunctions.GetStatsComponent` 0) (`|CreateDelegate` :!event `StatsUpdated`)))
  (set `self.CurrentHealth` (`self.MaxHealth`))
  (set `self.CurrentShield` (`self.MaxShield`)))

(fn `AddHealth`
  (params (Delta :type "Float (double-precision)") (HealthAdditionType :type "/Game/Blueprint/HealthSystem/Enum/E_HealthAdditionType Enum" :default "NewEnumerator0"))
  (bind _output_get (set `self.CurrentHealth` (`KismetMathLibrary.FClamp` (+ (`self.CurrentHealth`) (* Delta (select `/Game/Blueprint/HealthSystem/Enum/E_HealthAdditionType` HealthAdditionType :`NewEnumerator0` -1.0 :`NewEnumerator1` 1.0 :!type "Float (single-precision)"))) 0.0 (`self.MaxHealth`))))
  (if (== _output_get 0.0)
    (`self.OwnerOnDestroy`)))

(fn `StatsUpdated`
  (params (Stats :type "Map of /Game/Blueprint/InventoryEquipmentSystem/Enum/E_StatType Enum to Float (double-precision)"))
  (set `self.MaxHealth` (`BlueprintMapLibrary.Map_Find` Stats "NewEnumerator2"))
  (set `self.MaxShield` (`BlueprintMapLibrary.Map_Find` Stats "NewEnumerator3")))