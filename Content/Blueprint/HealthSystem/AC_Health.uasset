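; Actor component that tracks the owning actor's current and maximum health and shield.
; On BeginPlay it reads both maximums from the owner's stats component, starts full, and binds to stat updates to refresh the maximums.
; AddHealth and AddShield apply damage or regeneration as clamped, signed deltas, with no spillover between the pools.
; When health reaches zero, it calls CallOwnerOnDestroy.
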(event `self.ReceiveBeginPlay`
  (bind _statscomponent (message `/Game/Blueprint/HealthSystem/Interface/BPI_HealthInterface.GetStatsComponent` (`self.GetOwner`)))
  (add `/Game/Blueprint/StatSystem/AC_Stats.StatsUpdated` _statscomponent (`|CreateDelegate` :!event `StatsUpdated`))
  (bind _output_get (set `self.MaxHealth` (`/Game/Blueprint/StatSystem/AC_Stats.GetStat` _statscomponent "NewEnumerator2")))
  (set `self.CurrentHealth` _output_get)
  (bind _output_get_2 (set `self.MaxShield` (`/Game/Blueprint/StatSystem/AC_Stats.GetStat` _statscomponent "NewEnumerator3")))
  (set `self.CurrentShield` _output_get_2))

(fn `AddHealth`
  (params (Delta :type "Float (double-precision)") (HealthAdditionType :type "/Game/Blueprint/HealthSystem/Enum/E_HealthAdditionType Enum" :default "NewEnumerator0"))
  (bind _output_get (set `self.CurrentHealth` (`KismetMathLibrary.FClamp` (+ (`self.CurrentHealth`) (* Delta (select `/Game/Blueprint/HealthSystem/Enum/E_HealthAdditionType` HealthAdditionType :`NewEnumerator0` -1.0 :`NewEnumerator1` 1.0 :!type "Float (single-precision)"))) 0.0 (`self.MaxHealth`))))
  (if (== _output_get 0.0)
    (`self.OwnerOnDestroy`)))

(fn `AddShield`
  (params (Delta :type "Float (double-precision)") (ShieldAdditionType :type "/Game/Blueprint/HealthSystem/Enum/E_HealthAdditionType Enum" :default "NewEnumerator0"))
  (set `self.CurrentShield` (`KismetMathLibrary.FClamp` (+ (`self.CurrentShield`) (* Delta (select `/Game/Blueprint/HealthSystem/Enum/E_HealthAdditionType` ShieldAdditionType :`NewEnumerator0` -1.0 :`NewEnumerator1` 1.0 :!type "Float (single-precision)"))) 0.0 (`self.MaxShield`))))

(fn `StatsUpdated`
  (params (Stats :type "Map of /Game/Blueprint/InventoryEquipmentSystem/Enum/E_StatType Enum to Float (double-precision)"))
  (set `self.MaxHealth` (`BlueprintMapLibrary.Map_Find` Stats "NewEnumerator2"))
  (set `self.MaxShield` (`BlueprintMapLibrary.Map_Find` Stats "NewEnumerator3")))