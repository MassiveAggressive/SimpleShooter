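; BP_InGamePlayerController is the in-game player controller that owns the player's inventory/equipment and stats components.
; When the inventory/equipment component fires StatsUpdated, it passes those stats to the stats component's AddStats with a fixed source enum.
; AddItem forwards to the inventory component, and getters expose the inventory/equipment and stats components, while GetSkillComponent returns nothing.
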(event `self.AC_InventoryEquipment.StatsUpdated`
  (params (Stats :type "Map of /Game/Blueprint/InventoryEquipmentSystem/Enum/E_StatType Enum to /Game/Blueprint/InventoryEquipmentSystem/Struct/S_StatAmount Structure" :default _))
  (`/Game/Blueprint/StatSystem/AC_Stats.AddStats` (`self.AC_Stats`) "NewEnumerator0" Stats))

(fn `AddItem`
  (params (Item :type "/Game/Blueprint/InventoryEquipmentSystem/Struct/S_Item Structure"))
  (returns (Added :type Boolean))
  (bind _added (`/Game/Blueprint/InventoryEquipmentSystem/AC_InventoryEquipment.AddItemToInventory` (`self.AC_InventoryEquipment`) Item))
  (return _added))

(fn `GetInventoryEquipmentComponent`
  (returns (InventoryEquipmentComponent :type "/Game/Blueprint/InventoryEquipmentSystem/AC_InventoryEquipment Object Reference"))
  (return (`self.AC_InventoryEquipment`)))

(fn `GetSkillComponent`
  (returns (SkillComponent :type "/Game/Blueprint/SkillSystem/AC_Skill Object Reference"))
  (return null))

(fn `GetStatsComponent`
  (returns (StatsComponent :type "/Game/Blueprint/StatSystem/AC_Stats Object Reference"))
  (return (`self.AC_Stats`)))

(fn `UserConstructionScript`
  (`parent.UserConstructionScript`))