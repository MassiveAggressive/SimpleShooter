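; BP_PlayerUnit is the player-controlled unit, with world-axis movement input and yaw-only facing toward a hit-result location each tick.
; On BeginPlay it creates the W_PlayerMain widget with a reference to itself and adds it to the viewport.
; Left mouse press constructs a WorldObject and prints its name.
; AddItem forwards the item to the controller's AddItemMessage and returns the result.
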(event `self.ReceiveBeginPlay`
  (`parent.ReceiveBeginPlay`)
  (bind _returnvalue (`|CreateWidget` "/Game/Blueprint/Player/Widget/W_PlayerMain.W_PlayerMain_C" null self))
  (bind _output_get (set `self.W_PlayerMain` _returnvalue))
  (`UserWidget.AddToViewport` _output_get 0))

(event `Key|LeftMouseButton`
  (params (Key :type "Key Structure"))
  (:`Pressed`
    (bind _returnvalue (`|GenericCreateObject` "/Script/SimpleShooter.WorldObject"))
    (`KismetSystemLibrary.PrintString` (`KismetSystemLibrary.GetDisplayName` _returnvalue))))

(event `self.ReceiveTick`
  (params (DeltaSeconds :type "Float (single-precision)"))
  (bind (_returnvalue_roll _returnvalue_pitch _returnvalue_yaw) (`KismetMathLibrary.BreakRotator` (`KismetMathLibrary.FindLookAtRotation` (`self.K2_GetActorLocation`) (`/Game/Blueprint/GeneralFunctions.GetHitResult`))))
  (`self.K2_SetActorRotation` (`KismetMathLibrary.MakeRotator` 0.0 0.0 _returnvalue_yaw)))

(event `InputAxis|MoveForward`
  (params (AxisValue :type "Float (single-precision)"))
  (`self.AddMovementInput` (1.0 0.0 0.0) AxisValue))

(event `InputAxis|MoveRight`
  (params (AxisValue :type "Float (single-precision)"))
  (`self.AddMovementInput` (0.0 1.0 0.0) AxisValue))

(fn `AddItem`
  (params (Item :type "/Game/Blueprint/InventoryEquipmentSystem/Struct/S_Item Structure"))
  (returns (Added :type Boolean))
  (bind _added (message `/Game/Blueprint/Player/Interface/BPI_Equipment.AddItem` (`self.GetController`) Item))
  (return _added))

(fn `UserConstructionScript`
  (`parent.UserConstructionScript`))