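; AC_Skill is a skill component that creates the skill tree widget, registers available skills and activates them.
; On start it walks linked DT_Skill rows recursively from RegenerateHealth, filling SkillMap and announcing each addition.
; UseSkill spawns a skill actor, seeking its affected object on the player pawn or equipment inventory.
; Skills lacking a target wait in RelatedObjects until ObjectsFound initializes them with a matching-class object.
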(event `self.ReceiveBeginPlay`
  (bind _returnvalue (`|CreateWidget` "/Game/Blueprint/SkillSystem/Widget/W_SkillTree.W_SkillTree_C" null self))
  (bind _output_get (set `self.W_SkillTree` _returnvalue))
  (message `/Game/Blueprint/Widget/Interface/BPI_MainWidget.AddWidget` (`/Game/Blueprint/GeneralFunctions.GetWidget`) _output_get)
  (`self.Initialize`))

(fn `AddSkill`
  (params (Skill :type "/Game/Blueprint/SkillSystem/Struct/S_Skill Structure"))
  (locals (SkillArrayRef :type "Array of /Game/Blueprint/SkillSystem/Struct/S_Skill Structure"))
  (bind _skill (`local.Skill`))
  (bind ((`Class_11_960592F0462214129258659E2FDF113C` _class) (`NextSkills_22_E317F3E148A927B89FF0A9B0DC1CCA48` _nextskills)) (break `/Game/Blueprint/SkillSystem/Struct/S_Skill` _skill))
  (bind (_datatable _rowname) (break `DataTableRowHandle` _nextskills))
  (if (not (`.ReturnValue` (`BlueprintMapLibrary.Map_Find` (`self.SkillMap`) (`.Class_11_960592F0462214129258659E2FDF113C` (break `/Game/Blueprint/SkillSystem/Struct/S_Skill` Skill)))))
    (`BlueprintMapLibrary.Map_Add` (`self.SkillMap`) _class _skill)
    (`self.SkillAdded` _skill)
    (bind _returnvalue (`|GetDataTableRow` _datatable _rowname)
      (:`then`
        (`self.AddSkill` _returnvalue)))))

(fn `Initialize`
  (bind _returnvalue (`|GetDataTableRow` "/Game/Blueprint/SkillSystem/DT_Skill.DT_Skill" "RegenerateHealth")
    (:`then`
      (`self.AddSkill` _returnvalue))))

(fn `ObjectsFound`
  (params (Object :type "Object Object Reference"))
  (bind _keys (`BlueprintMapLibrary.Map_Keys` (`self.RelatedObjects`)))
  (for _array_element _keys
    (if (`KismetMathLibrary.ClassIsChildOf` (`GameplayStatics.GetObjectClass` Object) _array_element)
      (`/Game/Blueprint/SkillSystem/Skill/BP_SkillBase.Initialize` (`BlueprintMapLibrary.Map_Find` (`self.RelatedObjects`) _array_element) (`local.Object`))
      (`BlueprintMapLibrary.Map_Remove` (`self.RelatedObjects`) _array_element)
      (break)))
  (return))

(fn `UseSkill`
  (params (Skill :type "/Game/Blueprint/SkillSystem/Skill/BP_SkillBase Class Reference"))
  (locals (UsedSkillClassRef :type "/Game/Blueprint/SkillSystem/Skill/BP_SkillBase Class Reference") (UsedSkillRef :type "/Game/Blueprint/SkillSystem/Struct/S_Skill Structure") (ObjectFoundRef :type Boolean :default false) (SpawnedSkillRef :type "/Game/Blueprint/SkillSystem/Skill/BP_SkillBase Object Reference"))
  (bind _skill (`local.Skill`))
  (set `local.UsedSkillClassRef` Skill)
  (bind _output_get (set `local.UsedSkillRef` (`BlueprintMapLibrary.Map_Find` (`self.SkillMap`) Skill)))
  (bind ((`AffectedObjectLocation_25_8C85C88B4C3C0350F1B93FAD6B073234` _affectedobjectlocation) (`AffectedObjectClass_29_99D561F24D2AC9AE5050349F86501D88` _affectedobjectclass)) (break `/Game/Blueprint/SkillSystem/Struct/S_Skill` _output_get))
  (bind (_objects _found) (message `/Game/Blueprint/SkillSystem/Interface/BPI_ObjectHost.GetRelatedObjectsOrBind` (select `/Game/Blueprint/SkillSystem/Enum/E_AffectedObjectLocation` _affectedobjectlocation :`NewEnumerator0` (`GameplayStatics.GetPlayerPawn` 0) :`NewEnumerator1` (`/Game/Blueprint/Player/BP_InGamePlayerController.AC_InventoryEquipment` (`/Game/Blueprint/GeneralFunctions.GetInGamePlayerController` 0)) :!type "Object Object Reference") _affectedobjectclass self))
  (set `local.ObjectFoundRef` _found)
  (bind _returnvalue (`|SpawnActorFromClass` (`local.UsedSkillClassRef`) (`KismetMathLibrary.MakeTransform` (0.0 0.0 0.0)) "AlwaysSpawn" "OverrideRootScale" null (`|GetArrayItem` _objects) (struct) null))
  (set `local.SpawnedSkillRef` _returnvalue)
  (if (`local.ObjectFoundRef`)
    (`BlueprintMapLibrary.Map_Add` (`self.UsedSkillsRefs`) (`local.Skill`) (`local.SpawnedSkillRef`))
    (`BlueprintMapLibrary.Map_Add` (`self.UsedSkills`) _skill (`BlueprintMapLibrary.Map_Find` (`self.SkillMap`) _skill))
    (else
      (`BlueprintMapLibrary.Map_Add` (`self.RelatedObjects`) (`.AffectedObjectClass_29_99D561F24D2AC9AE5050349F86501D88` (break `/Game/Blueprint/SkillSystem/Struct/S_Skill` (`local.UsedSkillRef`))) (`local.SpawnedSkillRef`)))))