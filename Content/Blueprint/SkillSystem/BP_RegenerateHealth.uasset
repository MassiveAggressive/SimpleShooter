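; BP_RegenerateHealth is a skill Blueprint that gives periodic health regeneration to the affected actor.
; Initialize calls the parent, caches the actor's AC_HealthComponent and activates the skill only if that component exists.
; Activation starts a looping timer with an interval of one over RegenerationRate, and deactivation clears it.
; ApplyAffect, the apparent timer callback, adds RegeneratedHealthAmount through the health component.
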(fn `ActivateSkill`
  (`parent.ActivateSkill`)
  (bind _returnvalue (`KismetSystemLibrary.K2_SetTimerDelegate` (`|CreateDelegate` :!event `ApplyAffect`) (/ 1.0 (`self.RegenerationRate`)) true))
  (set `self.RegenerationTimer` _returnvalue))

(fn `ApplyAffect`
  (`parent.ApplyAffect`)
  (`/Game/Blueprint/HealthSystem/AC_HealthComponent.AddHealth` (`self.AffectedComponent`) (`self.RegeneratedHealthAmount`) "NewEnumerator1"))

(fn `DeactivateSkill`
  (`parent.DeactivateSkill`)
  (`KismetSystemLibrary.K2_ClearAndInvalidateTimerHandle` (`self.RegenerationTimer`)))

(fn `Initialize`
  (params (AffectedActor :type "Actor Object Reference"))
  (bind _returnvalue (`self.GetComponentByClass` AffectedActor "/Game/Blueprint/HealthSystem/AC_HealthComponent.AC_HealthComponent_C"))
  (`parent.Initialize` AffectedActor)
  (`/Engine/EditorBlueprintResources/StandardMacros.IsValid` _returnvalue
    (:`Is Valid`
      (set `self.AffectedComponent` _returnvalue)
      (`self.ActivateSkill`))))

(fn `UserConstructionScript`
  (`parent.UserConstructionScript`))