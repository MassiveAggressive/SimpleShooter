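; BP_ShootBonus is a weapon skill that fires an extra shot after every set number of regular shots.
; On initialization it casts the affected actor to BP_WeaponBase, then activates and binds to the weapon's Shooted event to count shots.
; At the threshold, a timer schedules the bonus shot half a fire interval later.
; Bonus shots are flagged as skill-affected, so the counter ignores them and cannot self-trigger.
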(event `CustomEvent`
  (`/Game/Blueprint/InventoryEquipmentSystem/Item/Weapon/BP_WeaponBase.Shoot` (`self.AffectedWeapon`) true))

(fn `ActivateSkill`
  (`parent.ActivateSkill`)
  (add `/Game/Blueprint/InventoryEquipmentSystem/Item/Weapon/BP_WeaponBase.Shooted` (`self.AffectedWeapon`) (`|CreateDelegate` :!event `OnShoot`)))

(fn `ApplyAffect`
  (`parent.ApplyAffect`)
  (`KismetSystemLibrary.K2_SetTimerDelegate` (`|CreateDelegate` :!event `CustomEvent`) (/ (/ 1.0 (`/Game/Blueprint/InventoryEquipmentSystem/Item/Weapon/BP_WeaponBase.FireRate` (`self.AffectedWeapon`))) 2.0)))

(fn `Initialize`
  (params (AffectedActor :type "Actor Object Reference"))
  (`parent.Initialize` AffectedActor)
  (bind _asbp_weapon_base (cast `/Game/Blueprint/InventoryEquipmentSystem/Item/Weapon/BP_WeaponBase` AffectedActor))
  (set `self.AffectedWeapon` _asbp_weapon_base)
  (`self.ActivateSkill`))

(fn `OnShoot`
  (params (AffectedBySkill :type Boolean))
  (if (not AffectedBySkill)
    (bind _result (`/Engine/EditorBlueprintResources/StandardMacros.IncrementInt` (`self.ShootCounter`))
      (:`  `
        (if (== _result (`self.ShootCountForAffect`))
          (`self.ApplyAffect`)
          (set `self.ShootCounter` 0))))))

(fn `UserConstructionScript`
  (`parent.UserConstructionScript`))