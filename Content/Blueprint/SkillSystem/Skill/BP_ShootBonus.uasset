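; BP_ShootBonus is a weapon skill that grants a bonus shot after a set number of regular shots.
; It finds its target weapon among the inventory equipment component's spawned items or on item spawn, then activates by binding to that weapon's shot event.
; A counter ignores skill-triggered shots, and at the threshold a timer fires the extra shot half a fire interval later, flagged as skill-affected.
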(event `self.ReceiveBeginPlay`
  (bind _inventoryequipmentcomponent (message `/Game/Blueprint/Player/Interface/BPI_InGamePlayerController.GetInventoryEquipmentComponent` (`GameplayStatics.GetPlayerController` 0)))
  (add `/Game/Blueprint/InventoryEquipmentSystem/AC_InventoryEquipment.ItemSpawned` _inventoryequipmentcomponent (`|CreateDelegate` :!event `OnItemSpawned`))
  (bind _spawneditems (`/Game/Blueprint/InventoryEquipmentSystem/AC_InventoryEquipment.SpawnedItems` _inventoryequipmentcomponent))
  (bind _keys (`BlueprintMapLibrary.Map_Keys` _spawneditems))
  (for _array_element _keys
    (if (`KismetMathLibrary.ClassIsChildOf` (`.AffectedObjectClass_29_99D561F24D2AC9AE5050349F86501D88` (break `/Game/Blueprint/SkillSystem/Struct/S_Skill` (`self.Skill`))) _array_element)
      (`self.Initialize` (`.ItemRef_2_CF80017747B800EB1CB8A98331FEBF1C` (break `/Game/Blueprint/InventoryEquipmentSystem/Struct/S_SpawnedItemInfo` (`|GetArrayItem` (`.ItemArray_4_A8CCE1494982686A8C1F4DB342B3828B` (break `/Game/Blueprint/InventoryEquipmentSystem/Struct/S_SpawnedItemArray` (`BlueprintMapLibrary.Map_Find` _spawneditems _array_element)))))))
      (break))))

(event `CustomEvent`
  (`/Game/Blueprint/InventoryEquipmentSystem/Item/Weapon/BP_WeaponBase.Shoot` (`self.AffectedWeapon`) true))

(fn `ActivateSkill`
  (`parent.ActivateSkill`)
  (add `/Game/Blueprint/InventoryEquipmentSystem/Item/Weapon/BP_WeaponBase.Shooted` (`self.AffectedWeapon`) (`|CreateDelegate` :!event `OnShoot`)))

(fn `ApplyAffect`
  (`parent.ApplyAffect`)
  (`KismetSystemLibrary.K2_SetTimerDelegate` (`|CreateDelegate` :!event `CustomEvent`) (/ (/ 1.0 (`/Game/Blueprint/InventoryEquipmentSystem/Item/Weapon/BP_WeaponBase.FireRate` (`self.AffectedWeapon`))) 2.0)))

(fn `Initialize`
  (params (AffectedActor :type "Actor Object Reference"))
  (`parent.Initialize` AffectedActor)
  (bind _asbp_weapon_base (cast `/Game/Blueprint/InventoryEquipmentSystem/Item/Weapon/BP_WeaponBase` AffectedActor))
  (set `self.AffectedWeapon` _asbp_weapon_base)
  (`self.ActivateSkill`))

(fn `OnItemSpawned`
  (params (SpawnedItem :type "/Game/Blueprint/InventoryEquipmentSystem/Item/BP_ItemBase Object Reference"))
  (if (`KismetMathLibrary.ClassIsChildOf` (`GameplayStatics.GetObjectClass` SpawnedItem) (`.AffectedObjectClass_29_99D561F24D2AC9AE5050349F86501D88` (break `/Game/Blueprint/SkillSystem/Struct/S_Skill` (`self.Skill`))))
    (`self.Initialize` (`local.SpawnedItem`))))

(fn `OnShoot`
  (params (AffectedBySkill :type Boolean))
  (if (not AffectedBySkill)
    (bind _result (`/Engine/EditorBlueprintResources/StandardMacros.IncrementInt` (`self.ShootCounter`))
      (:`  `
        (if (== _result (`self.ShootCountForAffect`))
          (`self.ApplyAffect`)
          (set `self.ShootCounter` 0))))))

(fn `UserConstructionScript`
  (`parent.UserConstructionScript`))