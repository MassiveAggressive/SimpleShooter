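; BP_RegenerateShield is a skill that periodically adds shield through an AC_Health component.
; BeginPlay passes the player pawn to Initialize, which casts that object directly to AC_Health and activates the skill only if the cast succeeds.
; Activation starts a looping timer at RegenerationRate, and deactivation clears it.
; ApplyAffect calls AddShield with RegenerationAmount, extending the parent skill's behavior like the other overrides.
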(event `self.ReceiveBeginPlay`
  (`parent.ReceiveBeginPlay`)
  (`self.Initialize` (`GameplayStatics.GetPlayerPawn` 0)))

(fn `ActivateSkill`
  (`parent.ActivateSkill`)
  (bind _returnvalue (`KismetSystemLibrary.K2_SetTimerDelegate` (`|CreateDelegate` :!event `ApplyAffect`) (`self.RegenerationRate`) true))
  (set `self.RegenerationTimer` _returnvalue))

(fn `ApplyAffect`
  (`parent.ApplyAffect`)
  (`/Game/Blueprint/HealthSystem/AC_Health.AddShield` (`self.AC_Health`) (`self.RegenerationAmount`) "NewEnumerator1"))

(fn `DeactivateSkill`
  (`parent.DeactivateSkill`)
  (`KismetSystemLibrary.K2_ClearAndInvalidateTimerHandle` (`self.RegenerationTimer`)))

(fn `Initialize`
  (params (AffectedObject :type "Object Object Reference"))
  (`parent.Initialize` AffectedObject)
  (bind _asac_health (cast `/Game/Blueprint/HealthSystem/AC_Health` AffectedObject))
  (set `self.AC_Health` _asac_health)
  (`self.ActivateSkill`))

(fn `UserConstructionScript`
  (`parent.UserConstructionScript`))