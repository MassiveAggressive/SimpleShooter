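; Dash skill actor that triggers a dash ability for the player when Left Shift is pressed.
; On BeginPlay it spawns a BP_DashAbility with the player character as the affected actor and binds a key-press event on the player controller base.
; OnKeyPressed filters for the hard-coded Left Shift key and calls Apply on the stored ability, which holds the dash logic outside this Blueprint.
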(event `self.ReceiveBeginPlay`
  (`parent.ReceiveBeginPlay`)
  (bind _returnvalue (`|SpawnActorFromClass` "/Game/Blueprint/AbilitySystem/BP_DashAbility.BP_DashAbility_C" (`KismetMathLibrary.MakeTransform` (0.0 0.0 0.0)) "AlwaysSpawn" "OverrideRootScale" null (`GameplayStatics.GetPlayerCharacter` 0) null))
  (set `self.BP_DashAbility` _returnvalue)
  (add `/Game/Blueprint/Player/BP_PlayerControllerBase.KeyPressed` (`/Game/Blueprint/GeneralFunctions.GetPlayerControllerBase` 0) (`|CreateDelegate` :!event `OnKeyPressed`)))

(fn `OnKeyPressed`
  (params (Key :type "Key Structure" :default "None"))
  (if (== Key "LeftShift")
    (`/Game/Blueprint/AbilitySystem/BP_AbilityBase.Apply` (`self.BP_DashAbility`))))

(fn `UserConstructionScript`
  (`parent.UserConstructionScript`))