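; AC_Stats is a stats component that combines stat bonuses from several sources into final values, readable through GetStat.
; AddStats stores stats per source, sums all sources by stat type and addition type, then broadcasts StatsUpdated.
; Only the first addition type's total feeds the final values.
; BeginPlay seeds hard-coded starting stats and creates a W_Stats widget bound to the component.
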(event `self.ReceiveBeginPlay`
  (`self.AddStats` "NewEnumerator1" (`|MakeMap` "NewEnumerator0" (make `/Game/Blueprint/InventoryEquipment/Struct/S_StatAmount` (`|MakeMap` "NewEnumerator0" 2.0 :!type "/Game/Blueprint/InventoryEquipment/Enum/E_StatAdditionType Enum" :!valuetype "Float (single-precision)")) "NewEnumerator1" (make `/Game/Blueprint/InventoryEquipment/Struct/S_StatAmount` (`|MakeMap` "NewEnumerator0" 100.0 :!type "/Game/Blueprint/InventoryEquipment/Enum/E_StatAdditionType Enum" :!valuetype "Float (single-precision)")) "NewEnumerator2" (make `/Game/Blueprint/InventoryEquipment/Struct/S_StatAmount` (`|MakeMap` "NewEnumerator0" 1000.0 :!type "/Game/Blueprint/InventoryEquipment/Enum/E_StatAdditionType Enum" :!valuetype "Float (single-precision)")) "NewEnumerator3" (struct) "NewEnumerator4" (make `/Game/Blueprint/InventoryEquipment/Struct/S_StatAmount` (`|MakeMap` "NewEnumerator0" 500.0 :!type "/Game/Blueprint/InventoryEquipment/Enum/E_StatAdditionType Enum" :!valuetype "Float (single-precision)")) :!type "/Game/Blueprint/InventoryEquipment/Enum/E_StatType Enum"))
  (bind _returnvalue (`|CreateWidget` "/Game/Blueprint/Stat/Widget/W_Stats.W_Stats_C" null self))
  (bind _output_get (set `self.W_Stats` _returnvalue))
  (message `/Game/Blueprint/Widget/Interface/BPI_MainWidget.AddWidget` (`/Game/Blueprint/GeneralFunctions.GetWidget`) _output_get))

(fn `AddStats`
  (params (StatsFrom :type "/Game/Blueprint/Stat/Enum/E_StatsFrom Enum" :default "NewEnumerator0") (Stats :type "Map of /Game/Blueprint/InventoryEquipment/Enum/E_StatType Enum to /Game/Blueprint/InventoryEquipment/Struct/S_StatAmount Structure"))
  (locals (AddedStatsRef :type "Map of /Game/Blueprint/InventoryEquipment/Enum/E_StatType Enum to /Game/Blueprint/InventoryEquipment/Struct/S_StatAmount Structure") (FinalStatsRef :type "Map of /Game/Blueprint/InventoryEquipment/Enum/E_StatType Enum to /Game/Blueprint/InventoryEquipment/Struct/S_StatAmount Structure") (AddedStatAmountRef :type "Map of /Game/Blueprint/InventoryEquipment/Enum/E_StatAdditionType Enum to Float (double-precision)") (FinalStatAmountRef :type "Map of /Game/Blueprint/InventoryEquipment/Enum/E_StatAdditionType Enum to Float (double-precision)") (CurrentStatsFromRef :type "/Game/Blueprint/Stat/Enum/E_StatsFrom Enum") (CurrentStatTypeRef :type "/Game/Blueprint/InventoryEquipment/Enum/E_StatType Enum") (CurrentStatAdditionTypeRef :type "/Game/Blueprint/InventoryEquipment/Enum/E_StatAdditionType Enum"))
  (`BlueprintMapLibrary.Map_Add` (`self.AdditiveStatsMap`) StatsFrom (make `/Game/Blueprint/Stat/Struct/S_Stats` Stats))
  (bind _enumvalue (foreach `/Game/Blueprint/Stat/Enum/E_StatsFrom` false)
    (:`LoopBody`
      (bind _output_get (set `local.CurrentStatsFromRef` _enumvalue))
      (set `local.AddedStatsRef` (`.Stats_4_C407A5BD416712E751F687869426256B` (break `/Game/Blueprint/Stat/Struct/S_Stats` (`BlueprintMapLibrary.Map_Find` (`self.AdditiveStatsMap`) _output_get))))
      (bind _enumvalue_2 (foreach `/Game/Blueprint/InventoryEquipment/Enum/E_StatType` false)
        (:`LoopBody`
          (bind _output_get_2 (set `local.CurrentStatTypeRef` _enumvalue_2))
          (set `local.AddedStatAmountRef` (`.StatAdditionType_9_AAA81259450362BDB3A322B1F09E3D19` (break `/Game/Blueprint/InventoryEquipment/Struct/S_StatAmount` (`BlueprintMapLibrary.Map_Find` (`local.AddedStatsRef`) _output_get_2))))
          (set `local.FinalStatAmountRef` (`.StatAdditionType_9_AAA81259450362BDB3A322B1F09E3D19` (break `/Game/Blueprint/InventoryEquipment/Struct/S_StatAmount` (`BlueprintMapLibrary.Map_Find` (`local.FinalStatsRef`) _output_get_2))))
          (bind _enumvalue_3 (foreach `/Game/Blueprint/InventoryEquipment/Enum/E_StatAdditionType` false)
            (:`LoopBody`
              (bind _output_get_3 (set `local.CurrentStatAdditionTypeRef` _enumvalue_3))
              (`BlueprintMapLibrary.Map_Add` (`local.FinalStatAmountRef`) (`local.CurrentStatAdditionTypeRef`) (+ (`BlueprintMapLibrary.Map_Find` (`local.FinalStatAmountRef`) _output_get_3) (`BlueprintMapLibrary.Map_Find` (`local.AddedStatAmountRef`) _output_get_3))))
            (:`then`
              (`BlueprintMapLibrary.Map_Add` (`local.FinalStatsRef`) (`local.CurrentStatTypeRef`) (make `/Game/Blueprint/InventoryEquipment/Struct/S_StatAmount` (`local.FinalStatAmountRef`))))))))
    (:`then`
      (bind _enumvalue_4 (foreach `/Game/Blueprint/InventoryEquipment/Enum/E_StatType` false)
        (:`LoopBody`
          (set `local.CurrentStatTypeRef` _enumvalue_4)
          (`BlueprintMapLibrary.Map_Add` (`self.FinalStats`) (`local.CurrentStatTypeRef`) (`BlueprintMapLibrary.Map_Find` (`.StatAdditionType_9_AAA81259450362BDB3A322B1F09E3D19` (break `/Game/Blueprint/InventoryEquipment/Struct/S_StatAmount` (`BlueprintMapLibrary.Map_Find` (`local.FinalStatsRef`) _enumvalue_4))) "NewEnumerator0")))
        (:`then`
          (`self.StatsUpdated` (`self.FinalStats`)))))))

(fn `GetStat`
  (params (StatType :type "/Game/Blueprint/InventoryEquipment/Enum/E_StatType Enum" :default "NewEnumerator0"))
  (returns (StatAAmount :type "Float (double-precision)"))
  (return (`BlueprintMapLibrary.Map_Find` (`self.FinalStats`) StatType)))