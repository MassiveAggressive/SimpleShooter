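; Base weapon Blueprint that starts auto-firing on BeginPlay and broadcasts Shooted per shot, printing the interval for debugging.
; Construction resolves Projectile from the Ammo data table's related row and builds evenly spaced, centered arrow components as barrels, rebuilt when count or spacing changes.
; A looping timer paces shots from FireRate, which stat updates set.
; Mid-fire rate changes use a one-shot timer to preserve cooldown progress before looping resumes.
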(event `self.ReceiveBeginPlay`
  (`parent.ReceiveBeginPlay`)
  (`self.StartShooting`))

(event `SetShootAvailable`
  (set `self.IsShootAvailable` true)
  (if (`self.IsShooting`)
    (`self.Shoot` false)
    (else
      (`KismetSystemLibrary.K2_ClearAndInvalidateTimerHandle` (`self.ShootTimer`)))))

(event `Shoot`
  (params (AffectedBySkill :type Boolean))
  (bind _returnvalue (`GameplayStatics.GetTimeSeconds`))
  (set `self.IsShootAvailable` false)
  (`self.Shooted` AffectedBySkill)
  (`KismetSystemLibrary.PrintString` (`KismetStringLibrary.Conv_DoubleToString` (- _returnvalue (`self.Time`))) true true (struct :`G` 0.66 :`B` 1.0 :`A` 1.0) 20.0)
  (set `self.Time` _returnvalue))

(fn `AddBarrelDistance`
  (params (Delta :type "Float (double-precision)"))
  (bind _returnvalue (+ (`self.BarrelsDistance`) Delta))
  (set `self.BarrelsDistance` (`KismetMathLibrary.SelectFloat` 0.0 _returnvalue (<= _returnvalue 0.0)))
  (`self.HandleBarrelsVariablesChanged`))

(fn `AddBarrelsCount`
  (params (Delta :type Integer))
  (set `self.BarrelsCount` (+ (`self.BarrelsCount`) Delta))
  (`self.HandleBarrelsVariablesChanged`))

(fn `AddFireRate`
  (params (Delta :type "Float (double-precision)"))
  (set `self.FireRate` (+ (`self.FireRate`) Delta))
  (if (`self.IsShooting`)
    (`self.HandleFireRateChanged`)))

(fn `HandleBarrelsVariablesChanged`
  (bind _returnvalue (- (`self.BarrelsCount`) 1))
  (for _array_element (`self.Barrels`)
    (`ActorComponent.K2_DestroyComponent` _array_element))
  (`KismetArrayLibrary.Array_Clear` (`self.Barrels`))
  (for _index (range (+ _returnvalue 1))
    (bind _returnvalue_2 (`AddComponent|NODE_AddArrowComponent-2` :`RelativeTransform` (`KismetMathLibrary.MakeTransform` (`KismetMathLibrary.MakeVector` 0.0 (- (* _index (`self.BarrelsDistance`)) (/ (* _returnvalue (`self.BarrelsDistance`)) 2.0))))))
    (`KismetArrayLibrary.Array_Add` (`self.Barrels`) _returnvalue_2)))

(fn `HandleFireRateChanged`
  (bind _shoottimer (`self.ShootTimer`))
  (bind _returnvalue (select `bool` (`KismetSystemLibrary.K2_TimerExistsHandle` _shoottimer) :`false` (`self.NewShootTimer`) :`true` _shoottimer))
  (bind _returnvalue_2 (`KismetSystemLibrary.K2_GetTimerRemainingTimeHandle` _returnvalue))
  (bind _returnvalue_3 (`KismetSystemLibrary.K2_SetTimerDelegate` (`|CreateDelegate` :!event `SetNewShootTimer`) (* (/ 1.0 (`self.FireRate`)) (/ _returnvalue_2 (+ (`KismetSystemLibrary.K2_GetTimerElapsedTimeHandle` _returnvalue) _returnvalue_2)))))
  (set `self.NewShootTimer` _returnvalue_3)
  (`KismetSystemLibrary.K2_ClearAndInvalidateTimerHandle` (`self.ShootTimer`)))

(fn `OnStatsUpdated`
  (params (Stats :type "Map of /Game/Blueprint/InventoryEquipmentSystem/Enum/E_StatType Enum to Float (double-precision)" :default _))
  (`parent.OnStatsUpdated` Stats)
  (`self.SetFireRate` (`BlueprintMapLibrary.Map_Find` (`self.Stats`) "NewEnumerator0")))

(fn `SetBarrelDistance`
  (params (Value :type "Float (double-precision)"))
  (set `self.BarrelsDistance` (`KismetMathLibrary.SelectFloat` 0.0 Value (<= Value 0.0)))
  (`self.HandleBarrelsVariablesChanged`))

(fn `SetBarrelsCount`
  (params (Value :type Integer))
  (set `self.BarrelsCount` Value)
  (`self.HandleBarrelsVariablesChanged`))

(fn `SetFireRate`
  (params (Value :type "Float (double-precision)"))
  (set `self.FireRate` Value)
  (if (`self.IsShooting`)
    (`self.HandleFireRateChanged`)))

(fn `SetNewShootTimer`
  (bind _returnvalue (`KismetSystemLibrary.K2_SetTimerDelegate` (`|CreateDelegate` :!event `SetShootAvailable`) (/ 1.0 (`self.FireRate`)) true))
  (set `self.ShootTimer` _returnvalue)
  (`self.SetShootAvailable`))

(fn `StartShooting`
  (set `self.IsShooting` true)
  (if (`self.IsShootAvailable`)
    (`self.Shoot` false)
    (bind _returnvalue (`KismetSystemLibrary.K2_SetTimerDelegate` (`|CreateDelegate` :!event `SetShootAvailable`) (/ 1.0 (`self.FireRate`)) true))
    (set `self.ShootTimer` _returnvalue)))

(fn `StopShooting`
  (set `self.IsShooting` false))

(fn `UserConstructionScript`
  (bind (_datatable _rowname) (break `DataTableRowHandle` (`self.Ammo`)))
  (bind _returnvalue (- (`self.BarrelsCount`) 1))
  (bind _returnvalue_2 (`|GetDataTableRow` _datatable _rowname)
    (:`then`
      (bind (_datatable_2 _rowname_2) (break `DataTableRowHandle` (`|GetArrayItem` (`.RelatedTableRows_61_F435BFDE4D07AFFAC5CEED943A52A84D` (break `/Game/Blueprint/InventoryEquipmentSystem/Struct/S_Item` _returnvalue_2)))))
      (bind _returnvalue_3 (`|GetDataTableRow` _datatable_2 _rowname_2)
        (:`then`
          (set `self.Projectile` _returnvalue_3)
          (for _index (range (+ _returnvalue 1))
            (bind _returnvalue_4 (`AddComponent|NODE_AddArrowComponent-4` :`RelativeTransform` (`KismetMathLibrary.MakeTransform` (`KismetMathLibrary.MakeVector` 0.0 (- (* _index (`self.BarrelsDistance`)) (/ (* _returnvalue (`self.BarrelsDistance`)) 2.0))))))
            (`KismetArrayLibrary.Array_Add` (`self.Barrels`) _returnvalue_4)))))))