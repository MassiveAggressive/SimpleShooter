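; BP_ProjectileBase is a base projectile actor in the inventory equipment system that deals damage on impact.
; The construction script applies the Projectile data to its box, mesh, tinted dynamic material and initial speed, and blocks only the configured collision channels.
; On hit, it sends DamageAmount through BPI_HealthInterface to actors implementing it, spawns color-matched Niagara sparks along the hit normal, then destroys itself.
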(event `self.Box.OnComponentHit`
  (params (HitComponent :type "PrimitiveComponent Object Reference") (OtherActor :type "Actor Object Reference") (OtherComp :type "PrimitiveComponent Object Reference") (NormalImpulse :type "Vector Structure") (Hit :type "HitResult Structure (by ref)"))
  (bind (_bblockinghit _binitialoverlap _time _distance _location _impactpoint _normal) (`GameplayStatics.BreakHitResult` Hit))
  (if (`KismetSystemLibrary.DoesImplementInterface` OtherActor "/Game/Blueprint/HealthSystem/Interface/BPI_HealthInterface.BPI_HealthInterface_C")
    (message `/Game/Blueprint/HealthSystem/Interface/BPI_HealthInterface.AddHealth` OtherActor (`self.DamageAmount`) "NewEnumerator0"))
  (bind _returnvalue (`NiagaraFunctionLibrary.SpawnSystemAtLocation` "/Game/Asset/Particle/NS_Sparks.NS_Sparks" _location (`KismetMathLibrary.Conv_VectorToRotator` _normal)))
  (`FXSystemComponent.SetColorParameter` _returnvalue "Color" (`.Color_11_78122AF140D7E77A80655AA0077648A0` (break `/Game/Blueprint/InventoryEquipmentSystem/Item/Projectile/Struct/S_Projectile` (`self.Projectile`))))
  (`self.K2_DestroyActor`))

(fn `UserConstructionScript`
  (bind _staticmesh (`self.StaticMesh`))
  (bind _box (`self.Box`))
  (bind (_defaultsize _defaultscale _mesh _materialinstance _color _projectilespeed) (break `/Game/Blueprint/InventoryEquipmentSystem/Item/Projectile/Struct/S_Projectile` (`self.Projectile`)))
  (`BoxComponent.SetBoxExtent` (`self.Box`) _defaultsize true)
  (`SceneComponent.SetRelativeScale3D` _staticmesh _defaultscale)
  (`StaticMeshComponent.SetStaticMesh` _staticmesh _mesh)
  (bind _returnvalue (`PrimitiveComponent.CreateDynamicMaterialInstance` _staticmesh 0 _materialinstance "None"))
  (`MaterialInstanceDynamic.SetVectorParameterValue` _returnvalue "Color" _color)
  (set `ProjectileMovementComponent.InitialSpeed` _projectilespeed (`self.ProjectileMovement`))
  (`PrimitiveComponent.SetCollisionObjectType` _box (`self.ObjectType`))
  (`PrimitiveComponent.SetCollisionResponseToAllChannels` _box "ECR_Ignore")
  (for _array_element (`self.BlockedChannels`)
    (`PrimitiveComponent.SetCollisionResponseToChannel` _box _array_element "ECR_Block")))