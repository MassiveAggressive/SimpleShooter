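; Inventory and equipment component that stores items by generated ID, moves them between inventory and size-limited equipment slots, and creates the inventory widget on BeginPlay.
; A location map drives lookups, and dispatchers broadcast each change.
; Equipping can spawn actors on player pawn sockets, sharing spawn-once actors by tracking item IDs, and adds item stats, which unequipping subtracts.
; Objects can request spawned actors by class or bind until one spawns.
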(event `self.ReceiveBeginPlay`
  (bind _returnvalue (`|CreateWidget` "/Game/Blueprint/InventoryEquipmentSystem/Widget/W_InventoryEquipment.W_InventoryEquipment_C" null self))
  (bind _output_get (set `self.InventoryEquipment` _returnvalue))
  (message `/Game/Blueprint/Widget/Interface/BPI_MainWidget.AddWidget` (`/Game/Blueprint/GeneralFunctions.GetWidget`) _output_get))

(fn `AddItemToEquipment`
  (params (Item :type "/Game/Blueprint/InventoryEquipmentSystem/Struct/S_Item Structure"))
  (returns (Added :type Boolean))
  (locals (ItemRef :type "/Game/Blueprint/InventoryEquipmentSystem/Struct/S_Item Structure") (ItemArrayRef :type "Array of /Game/Blueprint/InventoryEquipmentSystem/Struct/S_Item Structure") (AttachedMeshRef :type "MeshComponent Object Reference") (SpawnedItemRef :type "/Game/Blueprint/InventoryEquipmentSystem/Item/BP_ItemBase Object Reference") (SpawnedItemArrayRef :type "Array of /Game/Blueprint/InventoryEquipmentSystem/Item/BP_ItemBase Object Reference") (NumOfLinkedItemsRef :type Integer))
  (bind _itemref (`local.ItemRef`))
  (bind _itemref_2 (`local.ItemRef`))
  (bind ((`ID_2_589BC6FE44BDACD8DB675395C8DF38CD` _id) (`ItemEquipmentSlotType_34_A4050D754E69B308063D8EB655E7CDF2` _itemequipmentslottype)) (break `/Game/Blueprint/InventoryEquipmentSystem/Struct/S_Item` (`local.ItemRef`)))
  (bind _output_get (set `local.ItemRef` Item))
  (bind ((`ItemEquipmentSlotType_34_A4050D754E69B308063D8EB655E7CDF2` _itemequipmentslottype_2)) (break `/Game/Blueprint/InventoryEquipmentSystem/Struct/S_Item` _output_get))
  (`self.IsThereAvailableSlot_Mac` _itemequipmentslottype_2
    (:`ThereIs`
      (if (`.ShouldBeSpawned_52_222446CE4F622A6558B1DEBB2F2985AC` (break `/Game/Blueprint/InventoryEquipmentSystem/Struct/S_Item` (`local.ItemRef`)))
        (bind _newitem (`self.SpawnItem` (`local.ItemRef`)))
        (set `local.ItemRef` _newitem))
      (bind _output_get_2 (set `local.ItemArrayRef` (`.Array_3_D8F4B92644B6A86C14E317AFFC7FDD96` (break `/Game/Blueprint/InventoryEquipmentSystem/Struct/S_ItemArray` (`BlueprintMapLibrary.Map_Find` (`self.EquipmentArray`) _itemequipmentslottype_2)))))
      (`KismetArrayLibrary.Array_Add` _output_get_2 _itemref_2)
      (`BlueprintMapLibrary.Map_Add` (`self.EquipmentArray`) (`.ItemEquipmentSlotType_34_A4050D754E69B308063D8EB655E7CDF2` (break `/Game/Blueprint/InventoryEquipmentSystem/Struct/S_Item` _itemref_2)) (make `/Game/Blueprint/InventoryEquipmentSystem/Struct/S_ItemArray` (`local.ItemArrayRef`)))
      (`KismetArrayLibrary.Array_Clear` (`local.ItemArrayRef`))
      (`BlueprintMapLibrary.Map_Add` (`self.ItemLocations`) _id (make `/Game/Blueprint/InventoryEquipmentSystem/Struct/S_ItemLocation` "NewEnumerator1" _itemequipmentslottype))
      (`self.CalculateStats` _itemref)
      (`self.ItemAddedToEquipment` _itemref)
      (return true))
    (:`ThereIsnt`
      (return false))))

(fn `AddItemToInventory`
  (params (Item :type "/Game/Blueprint/InventoryEquipmentSystem/Struct/S_Item Structure"))
  (returns (Added :type Boolean))
  (locals (ItemRef :type "/Game/Blueprint/InventoryEquipmentSystem/Struct/S_Item Structure") (ItemArrayRef :type "Array of /Game/Blueprint/InventoryEquipmentSystem/Struct/S_Item Structure"))
  (bind _itemref (`local.ItemRef`))
  (bind ((`ID_2_589BC6FE44BDACD8DB675395C8DF38CD` _id)) (break `/Game/Blueprint/InventoryEquipmentSystem/Struct/S_Item` _itemref))
  (bind _output_get (set `local.ItemRef` Item))
  (if (== (`.ID_2_589BC6FE44BDACD8DB675395C8DF38CD` (break `/Game/Blueprint/InventoryEquipmentSystem/Struct/S_Item` _output_get)) -1)
    (setmembers `/Game/Blueprint/InventoryEquipmentSystem/Struct/S_Item` :`StructRef` (`local.ItemRef`) :`ID` (`self.CreateANewID`)))
  (`BlueprintMapLibrary.Map_Add` (`self.InventoryArray`) _id _itemref)
  (`BlueprintMapLibrary.Map_Add` (`self.ItemLocations`) _id (make `/Game/Blueprint/InventoryEquipmentSystem/Struct/S_ItemLocation`))
  (`self.ItemAddedToInventory` (`local.ItemRef`))
  (return true))

(fn `CalculateStats`
  (params (Item :type "/Game/Blueprint/InventoryEquipmentSystem/Struct/S_Item Structure (by ref)") (WasEquipped :type Boolean :default true))
  (locals (StatAmountRef :type "Map of /Game/Blueprint/InventoryEquipmentSystem/Enum/E_StatAdditionType Enum to Float (double-precision)") (StatRef :type "/Game/Blueprint/InventoryEquipmentSystem/Struct/S_Stat Structure"))
  (bind ((`StatType_2_52DA18AC43F5B202D2BFB2B01AA6E3DA` _stattype) (`StatAdditionType_5_AEBBF82D44309CDAF5D07DA9313B4B85` _statadditiontype)) (break `/Game/Blueprint/InventoryEquipmentSystem/Struct/S_Stat` (`local.StatRef`)))
  (for _array_element (`.Stats_27_39E6F381494FC358CD3C8EB7B5FB155E` (break `/Game/Blueprint/InventoryEquipmentSystem/Struct/S_Item` Item))
    (bind _output_get (set `local.StatRef` _array_element))
    (bind (_stattype_2 _statadditiontype_2 _statamount) (break `/Game/Blueprint/InventoryEquipmentSystem/Struct/S_Stat` _output_get))
    (bind _output_get_2 (set `local.StatAmountRef` (`.StatAdditionType_9_AAA81259450362BDB3A322B1F09E3D19` (break `/Game/Blueprint/InventoryEquipmentSystem/Struct/S_StatAmount` (`BlueprintMapLibrary.Map_Find` (`self.Stats`) _stattype_2)))))
    (`BlueprintMapLibrary.Map_Add` (`local.StatAmountRef`) _statadditiontype (+ (`BlueprintMapLibrary.Map_Find` _output_get_2 _statadditiontype_2) (* _statamount (`KismetMathLibrary.SelectFloat` 1.0 -1.0 (`local.WasEquipped`)))))
    (`BlueprintMapLibrary.Map_Add` (`self.Stats`) _stattype (make `/Game/Blueprint/InventoryEquipmentSystem/Struct/S_StatAmount` (`local.StatAmountRef`))))
  (`self.StatsUpdated` (`self.Stats`)))

(fn `CheckIsItemValid`
  (params (ID :type Integer))
  (returns (IsValid :type Boolean) (ItemLocation :type "/Game/Blueprint/InventoryEquipmentSystem/Struct/S_ItemLocation Structure"))
  (bind (_value _returnvalue) (`BlueprintMapLibrary.Map_Find` (`self.ItemLocations`) ID))
  (return _returnvalue _value))

(fn `CreateANewID`
  (returns (NewID :type Integer))
  (bind _keys (`BlueprintMapLibrary.Map_Keys` (`self.ItemLocations`)))
  (return (`KismetMathLibrary.SelectInt` 0 (+ (`.MaxValue` (`KismetMathLibrary.MaxOfIntArray` _keys)) 1) (== (`KismetArrayLibrary.Array_Length` _keys) 0))))

(fn `DestroyItem`
  (params (Item :type "/Game/Blueprint/InventoryEquipmentSystem/Struct/S_Item Structure"))
  (locals (ItemRef :type "/Game/Blueprint/InventoryEquipmentSystem/Struct/S_Item Structure") (S_SpawnedItemArrayRef :type "Array of /Game/Blueprint/InventoryEquipmentSystem/Struct/S_SpawnedItemInfo Structure") (ItemIDsRef :type "Array of Integer"))
  (bind _itemidsref (`local.ItemIDsRef`))
  (bind _s_spawneditemarrayref (`local.S_SpawnedItemArrayRef`))
  (bind ((`Class_45_31B8AFB645AFF9B1B960DBBDC32EB92C` _class) (`SpawnedItem_55_D43AF61A4BAACACB9955BE8DE8486182` _spawneditem)) (break `/Game/Blueprint/InventoryEquipmentSystem/Struct/S_Item` (`local.ItemRef`)))
  (bind _output_get (set `local.ItemRef` Item))
  (bind _output_get_2 (set `local.S_SpawnedItemArrayRef` (`.ItemArray_4_A8CCE1494982686A8C1F4DB342B3828B` (break `/Game/Blueprint/InventoryEquipmentSystem/Struct/S_SpawnedItemArray` (`BlueprintMapLibrary.Map_Find` (`self.SpawnedItems`) (`.Class_45_31B8AFB645AFF9B1B960DBBDC32EB92C` (break `/Game/Blueprint/InventoryEquipmentSystem/Struct/S_Item` _output_get)))))))
  (if (`.ShouldBeSpawnedOnce_51_E6B65BA6463B573E3B775F82044D87BE` (break `/Game/Blueprint/InventoryEquipmentSystem/Struct/S_Item` (`local.ItemRef`)))
    (bind _output_get_3 (set `local.ItemIDsRef` (`.ItemIDs_11_404C0F654A9DACB6610654870FE021A4` (break `/Game/Blueprint/InventoryEquipmentSystem/Struct/S_SpawnedItemInfo` (`|GetArrayItem` _output_get_2)))))
    (bind _returnvalue (`KismetArrayLibrary.Array_Find` _output_get_3 (`.ID_2_589BC6FE44BDACD8DB675395C8DF38CD` (break `/Game/Blueprint/InventoryEquipmentSystem/Struct/S_Item` (`local.ItemRef`)))))
    (if (!= _returnvalue -1)
      (`KismetArrayLibrary.Array_Remove` _itemidsref _returnvalue)
      (if (== (`KismetArrayLibrary.Array_Length` _itemidsref) 0)
        (`Actor.K2_DestroyActor` _spawneditem)
        (`BlueprintMapLibrary.Map_Remove` (`self.SpawnedItems`) _class)
        (else
          (`BlueprintMapLibrary.Map_Add` (`self.SpawnedItems`) _class (make `/Game/Blueprint/InventoryEquipmentSystem/Struct/S_SpawnedItemArray` (`local.S_SpawnedItemArrayRef`))))))
    (else
      (for (_array_element _array_index) (`local.S_SpawnedItemArrayRef`)
        (bind (_itemids _itemref) (break `/Game/Blueprint/InventoryEquipmentSystem/Struct/S_SpawnedItemInfo` _array_element))
        (if (== (`|GetArrayItem` _itemids) (`.ID_2_589BC6FE44BDACD8DB675395C8DF38CD` (break `/Game/Blueprint/InventoryEquipmentSystem/Struct/S_Item` (`local.ItemRef`))))
          (`Actor.K2_DestroyActor` _itemref)
          (`KismetArrayLibrary.Array_Remove` _s_spawneditemarrayref _array_index)
          (if (== (`KismetArrayLibrary.Array_Length` _s_spawneditemarrayref) 0)
            (`BlueprintMapLibrary.Map_Remove` (`self.SpawnedItems`) (`.Class_45_31B8AFB645AFF9B1B960DBBDC32EB92C` (break `/Game/Blueprint/InventoryEquipmentSystem/Struct/S_Item` (`local.ItemRef`))))
            (break)
            (else
              (break))))))))

(fn `FindItemWithID`
  (params (ID :type Integer))
  (returns (ItemLocation :type "/Game/Blueprint/InventoryEquipmentSystem/Struct/S_ItemLocation Structure") (Item :type "/Game/Blueprint/InventoryEquipmentSystem/Struct/S_Item Structure") (Found :type Boolean))
  (locals (ItemLocationRef :type "/Game/Blueprint/InventoryEquipmentSystem/Struct/S_ItemLocation Structure") (ItemRef :type "/Game/Blueprint/InventoryEquipmentSystem/Struct/S_Item Structure"))
  (bind _itemref (`local.ItemRef`))
  (bind (_value _returnvalue) (`BlueprintMapLibrary.Map_Find` (`self.ItemLocations`) ID))
  (if _returnvalue
    (bind _output_get (set `local.ItemLocationRef` _value))
    (bind (_itemlocation _itemequipmentslottype) (break `/Game/Blueprint/InventoryEquipmentSystem/Struct/S_ItemLocation` _output_get))
    (switch `/Game/Blueprint/InventoryEquipmentSystem/Enum/E_ItemLocation` _itemlocation
      (:`NewEnumerator0`
        (return (`local.ItemLocationRef`) (`BlueprintMapLibrary.Map_Find` (`self.InventoryArray`) (`local.ID`)) true))
      (:`NewEnumerator1`
        (for _array_element (`.Array_3_D8F4B92644B6A86C14E317AFFC7FDD96` (break `/Game/Blueprint/InventoryEquipmentSystem/Struct/S_ItemArray` (`BlueprintMapLibrary.Map_Find` (`self.EquipmentArray`) _itemequipmentslottype)))
          (if (== (`.ID_2_589BC6FE44BDACD8DB675395C8DF38CD` (break `/Game/Blueprint/InventoryEquipmentSystem/Struct/S_Item` _array_element)) (`local.ID`))
            (set `local.ItemRef` _array_element)
            (break)))
        (return (`local.ItemLocationRef`) _itemref (!= (`.ID_2_589BC6FE44BDACD8DB675395C8DF38CD` (break `/Game/Blueprint/InventoryEquipmentSystem/Struct/S_Item` _itemref)) -1))))
    (else
      (return (struct) (struct) false))))

(fn `GetRelatedObjectsOrBind`
  (params (ObjectClass :type "Object Class Reference") (BindedObject :type "Object Object Reference"))
  (returns (Objects :type "Array of Object Object Reference") (Found :type Boolean))
  (locals (RelatedObjectClassesArrayRef :type "Array of Object Class Reference") (RelatedObjectsArrayRef :type "Array of Actor Object Reference") (FoundRef :type Boolean))
  (bind _keys (`BlueprintMapLibrary.Map_Keys` (`self.SpawnedActors`)))
  (for _array_element _keys
    (if (`KismetMathLibrary.ClassIsChildOf` _array_element ObjectClass)
      (set `local.RelatedObjectsArrayRef` (`.Array_3_9DD950994DB267B1416CD3856D8A6687` (break `/Game/Blueprint/SkillSystem/Struct/S_ActorRefArray` (`BlueprintMapLibrary.Map_Find` (`self.SpawnedActors`) _array_element))))
      (set `local.FoundRef` true)
      (break)))
  (if (`local.FoundRef`)
    (return (`local.RelatedObjectsArrayRef`) true)
    (else
      (`BlueprintMapLibrary.Map_Add` (`self.BindedRelatedObjects`) (`local.ObjectClass`) (`local.BindedObject`))
      (add `self.ItemSpawned` (`|CreateDelegate` :!event `OnItemSpawned`)))))

(fn `IsThereAvailableSlot`
  (params (SlotType :type "/Game/Blueprint/InventoryEquipmentSystem/Enum/E_ItemEquipmentSlotType Enum" :default "NewEnumerator5"))
  (returns (ReturnValue :type Boolean))
  (return (< (`KismetArrayLibrary.Array_Length` (`.Array_3_D8F4B92644B6A86C14E317AFFC7FDD96` (break `/Game/Blueprint/InventoryEquipmentSystem/Struct/S_ItemArray` (`BlueprintMapLibrary.Map_Find` (`self.EquipmentArray`) SlotType)))) (`BlueprintMapLibrary.Map_Find` (`self.EquipmentSlotsSizes`) SlotType))))

(fn `OnItemSpawned`
  (params (SpawnedItem :type "/Game/Blueprint/InventoryEquipmentSystem/Item/BP_ItemBase Object Reference"))
  (locals (SpawnedItemClassRef :type "/Game/Blueprint/InventoryEquipmentSystem/Item/BP_ItemBase Class Reference"))
  (set `local.SpawnedItemClassRef` (`GameplayStatics.GetObjectClass` SpawnedItem))
  (bind _keys (`BlueprintMapLibrary.Map_Keys` (`self.BindedRelatedObjects`)))
  (for _array_element _keys
    (if (`KismetMathLibrary.ClassIsChildOf` (`local.SpawnedItemClassRef`) _array_element)
      (message `/Game/Blueprint/SkillSystem/Interface/BPI_ObjectSeeker.ObjectsFound` (`BlueprintMapLibrary.Map_Find` (`self.BindedRelatedObjects`) _array_element) (`local.SpawnedItem`))
      (break))))

(fn `Send Item to Equipment`
  (params (ID :type Integer))
  (returns (Sended :type Boolean))
  (bind _id (`local.ID`))
  (bind (_itemlocation _item) (`self.FindItemWithID_Mac` ID)
    (:`Found`
      (switch `/Game/Blueprint/InventoryEquipmentSystem/Enum/E_ItemLocation` (`.ItemLocation_2_328BD9904C14A9B938144182DC00D9F5` (break `/Game/Blueprint/InventoryEquipmentSystem/Struct/S_ItemLocation` _itemlocation))
        (:`NewEnumerator0`
          (bind _added (`self.AddItemToEquipment` _item))
          (if _added
            (`BlueprintMapLibrary.Map_Remove` (`self.InventoryArray`) _id)
            (`self.ItemRemovedFromInventory` _id)
            (return true)
            (else
              _)))
        (:`NewEnumerator1`
          _)))
    (:`NotFound`
      _))
  (return false))

(fn `SendItemToInventory`
  (params (ID :type Integer))
  (returns (Sended :type Boolean))
  (locals (ItemArrayRef :type "Array of /Game/Blueprint/InventoryEquipmentSystem/Struct/S_Item Structure") (ItemRef :type "/Game/Blueprint/InventoryEquipmentSystem/Struct/S_Item Structure"))
  (bind _itemref (`local.ItemRef`))
  (bind (_itemlocation _item) (`self.FindItemWithID_Mac` ID)
    (:`Found`
      (set `local.ItemRef` _item)
      (switch `/Game/Blueprint/InventoryEquipmentSystem/Enum/E_ItemLocation` (`.ItemLocation_2_328BD9904C14A9B938144182DC00D9F5` (break `/Game/Blueprint/InventoryEquipmentSystem/Struct/S_ItemLocation` _itemlocation))
        (:`NewEnumerator0`
          _)
        (:`NewEnumerator1`
          (bind _added (`self.AddItemToInventory` _itemref))
          (if _added
            (bind _output_get (set `local.ItemArrayRef` (`.Array_3_D8F4B92644B6A86C14E317AFFC7FDD96` (break `/Game/Blueprint/InventoryEquipmentSystem/Struct/S_ItemArray` (`BlueprintMapLibrary.Map_Find` (`self.EquipmentArray`) (`.ItemEquipmentSlotType_34_A4050D754E69B308063D8EB655E7CDF2` (break `/Game/Blueprint/InventoryEquipmentSystem/Struct/S_Item` _itemref)))))))
            (for (_array_element _array_index) _output_get
              (bind _output_get_2 (set `local.ItemRef` _array_element))
              (if (== (`.ID_2_589BC6FE44BDACD8DB675395C8DF38CD` (break `/Game/Blueprint/InventoryEquipmentSystem/Struct/S_Item` _output_get_2)) (`local.ID`))
                (`KismetArrayLibrary.Array_Remove` (`local.ItemArrayRef`) _array_index)
                (`BlueprintMapLibrary.Map_Add` (`self.EquipmentArray`) (`.ItemEquipmentSlotType_34_A4050D754E69B308063D8EB655E7CDF2` (break `/Game/Blueprint/InventoryEquipmentSystem/Struct/S_Item` (`local.ItemRef`))) (make `/Game/Blueprint/InventoryEquipmentSystem/Struct/S_ItemArray` (`local.ItemArrayRef`)))
                (`self.DestroyItem` (`local.ItemRef`))
                (break)))
            (`self.CalculateStats` (`local.ItemRef`) false)
            (`self.ItemRemovedFromEquipment` (`local.ID`))
            (return true)
            (else
              _)))))
    (:`NotFound`
      _))
  (return false))

(fn `SpawnItem`
  (params (Item :type "/Game/Blueprint/InventoryEquipmentSystem/Struct/S_Item Structure"))
  (returns (NewItem :type "/Game/Blueprint/InventoryEquipmentSystem/Struct/S_Item Structure (by ref)"))
  (locals (ItemRef :type "/Game/Blueprint/InventoryEquipmentSystem/Struct/S_Item Structure") (SpawnedItemsArrayRef :type "Array of /Game/Blueprint/InventoryEquipmentSystem/Item/BP_ItemBase Object Reference") (AttachedMeshRef :type "MeshComponent Object Reference") (SpawnedItemRef :type "/Game/Blueprint/InventoryEquipmentSystem/Item/BP_ItemBase Object Reference") (S_SpawnedItemArrayRef :type "Array of /Game/Blueprint/InventoryEquipmentSystem/Struct/S_SpawnedItemInfo Structure") (NumOfLinkedItems :type Integer) (S_SpawnedItemInfoRef :type "/Game/Blueprint/InventoryEquipmentSystem/Struct/S_SpawnedItemInfo Structure") (SpawnedActorsArrayRef :type "Array of Actor Object Reference"))
  (bind _itemref (`local.ItemRef`))
  (bind _itemref_2 (`local.ItemRef`))
  (bind ((`ID_2_589BC6FE44BDACD8DB675395C8DF38CD` _id) (`Class_45_31B8AFB645AFF9B1B960DBBDC32EB92C` _class)) (break `/Game/Blueprint/InventoryEquipmentSystem/Struct/S_Item` _itemref_2))
  (bind ((`Class_45_31B8AFB645AFF9B1B960DBBDC32EB92C` _class_2)) (break `/Game/Blueprint/InventoryEquipmentSystem/Struct/S_Item` (`local.ItemRef`)))
  (bind _output_get (set `local.ItemRef` Item))
  (bind ((`ShouldBeSpawnedOnce_51_E6B65BA6463B573E3B775F82044D87BE` _shouldbespawnedonce) (`Class_45_31B8AFB645AFF9B1B960DBBDC32EB92C` _class_3)) (break `/Game/Blueprint/InventoryEquipmentSystem/Struct/S_Item` _output_get))
  (if (not (not _shouldbespawnedonce))
    (bind _output_get_2 (set `local.S_SpawnedItemArrayRef` (`.ItemArray_4_A8CCE1494982686A8C1F4DB342B3828B` (break `/Game/Blueprint/InventoryEquipmentSystem/Struct/S_SpawnedItemArray` (`BlueprintMapLibrary.Map_Find` (`self.SpawnedItems`) _class_3)))))
    (if (> (`KismetArrayLibrary.Array_Length` _output_get_2) 0)
      (bind _output_get_3 (set `local.S_SpawnedItemInfoRef` (`|GetArrayItem` (`local.S_SpawnedItemArrayRef`))))
      (bind (_itemids _itemref_3) (break `/Game/Blueprint/InventoryEquipmentSystem/Struct/S_SpawnedItemInfo` _output_get_3))
      (setmembers `/Game/Blueprint/InventoryEquipmentSystem/Struct/S_Item` :`StructRef` _itemref_2 :`SpawnedItem` _itemref_3)
      (`KismetArrayLibrary.Array_Add` _itemids _id)
      (`BlueprintMapLibrary.Map_Add` (`self.SpawnedItems`) _class (make `/Game/Blueprint/InventoryEquipmentSystem/Struct/S_SpawnedItemArray` (`local.S_SpawnedItemArrayRef`)))
      (return (`local.ItemRef`))
      (else
        _)))
  (bind (_mesh _sockettransform) (message `/Game/Blueprint/UnitBase/Interface/BPI_Unit.GetSocket` (`GameplayStatics.GetPlayerPawn` 0) (`.ItemEquipmentSlotType_34_A4050D754E69B308063D8EB655E7CDF2` (break `/Game/Blueprint/InventoryEquipmentSystem/Struct/S_Item` (`local.ItemRef`)))))
  (set `local.AttachedMeshRef` _mesh)
  (bind _returnvalue (`|SpawnActorFromClass` (`.Class_45_31B8AFB645AFF9B1B960DBBDC32EB92C` (break `/Game/Blueprint/InventoryEquipmentSystem/Struct/S_Item` (`local.ItemRef`))) _sockettransform "AlwaysSpawn" "OverrideRootScale" null _itemref null))
  (bind _output_get_4 (set `local.SpawnedItemRef` _returnvalue))
  (`Actor.K2_AttachToComponent` _output_get_4 (`local.AttachedMeshRef`) (`|GetEnumeratorName` (`.ItemEquipmentSlotType_34_A4050D754E69B308063D8EB655E7CDF2` (break `/Game/Blueprint/InventoryEquipmentSystem/Struct/S_Item` _itemref))) "SnapToTarget" "SnapToTarget" "SnapToTarget" true)
  (bind _output_get_5 (set `local.S_SpawnedItemArrayRef` (`.ItemArray_4_A8CCE1494982686A8C1F4DB342B3828B` (break `/Game/Blueprint/InventoryEquipmentSystem/Struct/S_SpawnedItemArray` (`BlueprintMapLibrary.Map_Find` (`self.SpawnedItems`) (`.Class_45_31B8AFB645AFF9B1B960DBBDC32EB92C` (break `/Game/Blueprint/InventoryEquipmentSystem/Struct/S_Item` (`local.ItemRef`))))))))
  (`KismetArrayLibrary.Array_Add` _output_get_5 (make `/Game/Blueprint/InventoryEquipmentSystem/Struct/S_SpawnedItemInfo` (`|MakeArray` (`.ID_2_589BC6FE44BDACD8DB675395C8DF38CD` (break `/Game/Blueprint/InventoryEquipmentSystem/Struct/S_Item` (`local.ItemRef`)))) (`local.SpawnedItemRef`)))
  (`BlueprintMapLibrary.Map_Add` (`self.SpawnedItems`) _class_2 (make `/Game/Blueprint/InventoryEquipmentSystem/Struct/S_SpawnedItemArray` (`local.S_SpawnedItemArrayRef`)))
  (bind _output_get_6 (set `local.SpawnedActorsArrayRef` (`.Array_3_9DD950994DB267B1416CD3856D8A6687` (break `/Game/Blueprint/SkillSystem/Struct/S_ActorRefArray` (`BlueprintMapLibrary.Map_Find` (`self.SpawnedActors`) _class_2)))))
  (`KismetArrayLibrary.Array_Add` _output_get_6 (`local.SpawnedItemRef`))
  (`BlueprintMapLibrary.Map_Add` (`self.SpawnedActors`) (`.Class_45_31B8AFB645AFF9B1B960DBBDC32EB92C` (break `/Game/Blueprint/InventoryEquipmentSystem/Struct/S_Item` (`local.ItemRef`))) (make `/Game/Blueprint/SkillSystem/Struct/S_ActorRefArray` (`local.SpawnedActorsArrayRef`)))
  (bind _structout (setmembers `/Game/Blueprint/InventoryEquipmentSystem/Struct/S_Item` :`StructRef` (`local.ItemRef`) :`SpawnedItem` (`local.SpawnedItemRef`)))
  (`self.ItemSpawned` (`local.SpawnedItemRef`))
  (return _structout))