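; BP_CollectableItem is a world pickup that gives its item to an overlapping actor and then removes itself.
; The construction script reads the item struct from a chosen data table row and sets the static mesh to its preview mesh.
; On box overlap it passes the item through the BPI_Equipment interface, destroying itself only if AddItemMessage returns true.
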(event `self.Box.OnComponentBeginOverlap`
  (params (OverlappedComponent :type "PrimitiveComponent Object Reference") (OtherActor :type "Actor Object Reference") (OtherComp :type "PrimitiveComponent Object Reference") (OtherBodyIndex :type Integer) (bFromSweep :type Boolean) (SweepResult :type "HitResult Structure (by ref)"))
  (if (`KismetSystemLibrary.DoesImplementInterface` OtherActor "/Game/Blueprint/Player/Interface/BPI_Equipment.BPI_Equipment_C")
    (bind _added (message `/Game/Blueprint/Player/Interface/BPI_Equipment.AddItem` OtherActor (`self.Item`)))
    (if _added
      (`self.K2_DestroyActor`))))

(fn `UserConstructionScript`
  (bind (_datatable _rowname) (break `DataTableRowHandle` (`self.ItemDataTableRow`)))
  (`parent.UserConstructionScript`)
  (bind _returnvalue (`|GetDataTableRow` _datatable _rowname)
    (:`then`
      (bind _output_get (set `self.Item` _returnvalue))
      (`StaticMeshComponent.SetStaticMesh` (`self.StaticMesh`) (`.PreviewMesh_49_5F30836F4BC2CECEB2799888AC76E3A1` (break `/Game/Blueprint/InventoryEquipment/Struct/S_Item` _output_get))))))