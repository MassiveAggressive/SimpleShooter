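; BP_BulletBase is a bullet actor, apparently a base for bullet types, that applies a health change to what it hits and destroys itself.
; On a Box hit, it sends DamageAmount through BPI_HealthInterface if the other actor implements it, then spawns Niagara sparks along the impact normal.
; The construction script creates a dynamic material for the Cube, so one Color variable tints both bullet and sparks.
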(event `self.Box.OnComponentHit`
  (params (HitComponent :type "PrimitiveComponent Object Reference") (OtherActor :type "Actor Object Reference") (OtherComp :type "PrimitiveComponent Object Reference") (NormalImpulse :type "Vector Structure") (Hit :type "HitResult Structure (by ref)"))
  (bind (_bblockinghit _binitialoverlap _time _distance _location _impactpoint _normal) (`GameplayStatics.BreakHitResult` Hit))
  (if (`KismetSystemLibrary.DoesImplementInterface` OtherActor "/Game/Blueprint/Health/BPI_HealthInterface.BPI_HealthInterface_C")
    (message `/Game/Blueprint/Health/BPI_HealthInterface.AddHealth` OtherActor (`self.DamageAmount`) "NewEnumerator0"))
  (bind _returnvalue (`NiagaraFunctionLibrary.SpawnSystemAtLocation` "/Game/Asset/Particle/NS_Sparks.NS_Sparks" _location (`KismetMathLibrary.Conv_VectorToRotator` _normal)))
  (`FXSystemComponent.SetColorParameter` _returnvalue "Color" (`self.Color`))
  (`self.K2_DestroyActor`))

(fn `UserConstructionScript`
  (bind _returnvalue (`PrimitiveComponent.CreateDynamicMaterialInstance` (`self.Cube`) 0 "/Game/Asset/Material/MI_Bullet.MI_Bullet" "None"))
  (bind _output_get (set `self.MaterialInstance` _returnvalue))
  (`MaterialInstanceDynamic.SetVectorParameterValue` _output_get "Color" (`self.Color`)))