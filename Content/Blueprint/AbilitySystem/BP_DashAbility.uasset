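; BP_DashAbility is an ability Blueprint that dashes the affected character in its current direction of movement.
; On BeginPlay it initializes with a valid AffectedActor, and Initialize casts that actor to Character and caches it.
; Apply launches the cached character along its normalized velocity scaled by DashSpeed, adding to existing velocity rather than overriding it, so a stationary character gets no dash.
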(event `self.ReceiveBeginPlay`
  (bind _affectedactor (`self.AffectedActor`))
  (`parent.ReceiveBeginPlay`)
  (`/Engine/EditorBlueprintResources/StandardMacros.IsValid` _affectedactor
    (:`Is Valid`
      (`self.Initialize` _affectedactor))))

(fn `Apply`
  (`parent.Apply`)
  (`Character.LaunchCharacter` (`self.AffectedCharacter`) (* (`KismetMathLibrary.Normal` (`self.GetVelocity` (`self.AffectedCharacter`))) (`self.DashSpeed`)) false false))

(fn `Initialize`
  (params (AffectedActor :type "Actor Object Reference"))
  (`parent.Initialize` AffectedActor)
  (bind _ascharacter (cast `Character` AffectedActor))
  (set `self.AffectedCharacter` _ascharacter))

(fn `UserConstructionScript`
  (`parent.UserConstructionScript`))