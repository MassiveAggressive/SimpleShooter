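; Particle-based weapon Blueprint that fires projectiles through a Niagara component, NSProjectile.
; Shoot and Stop switch firing on and off by setting the system's FireRate parameter.
; The construction script passes the Blueprint to Niagara as its Callback object.
; The ParticleData event increments a counter and prints it with the real time as debug output, without acting on any particle data.
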(event `Shoot`
  (`FXSystemComponent.SetFloatParameter` (`self.NS_Projectile`) "FireRate" 1.0))

(event `Stop`
  (`FXSystemComponent.SetFloatParameter` (`self.NS_Projectile`) "FireRate" 0.0))

(event `self.ReceiveParticleData`
  (params (Data :type "Array of BasicParticleData Structure (by ref)") (NiagaraSystem :type "NiagaraSystem Object Reference"))
  (bind _result (`/Engine/EditorBlueprintResources/StandardMacros.IncrementInt` (`self.Count`))
    (:`  `
      (`KismetSystemLibrary.PrintString` (`KismetStringLibrary.Concat_StrStr` (`KismetStringLibrary.Conv_DoubleToString` (`GameplayStatics.GetRealTimeSeconds`)) " | " (`KismetStringLibrary.Conv_IntToString` _result))))))

(fn `UserConstructionScript`
  (`NiagaraComponent.SetVariableObject` (`self.NS_Projectile`) "Callback" self))